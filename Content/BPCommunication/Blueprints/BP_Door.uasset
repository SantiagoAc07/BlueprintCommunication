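; BP_Door is a door actor that opens by hiding its Door component and dropping collision rather than animating.
; The OpenDoor and CloseDoor functions toggle the component's visibility and switch its collision between none and query-and-physics.
; A separate DoorOpen event also hides the component but disables collision on the whole actor, which CloseDoor does not re-enable.
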(event Custom|DoorOpen
  (Rendering|SetVisibility (Variables|Default|GetDoor) false false)
  (Collision|SetActorEnableCollision false))

(fn ConstructionScript)

(fn OpenDoor
  (Rendering|SetVisibility (Variables|Default|GetDoor) false false)
  (Collision|SetCollisionEnabled (Variables|Default|GetDoor) "NoCollision"))

(fn CloseDoor
  (Rendering|SetVisibility (Variables|Default|GetDoor) true false)
  (Collision|SetCollisionEnabled (Variables|Default|GetDoor) "QueryAndPhysics"))